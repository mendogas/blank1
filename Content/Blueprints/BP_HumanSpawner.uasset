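; BP_HumanSpawner is an actor that populates the level with humans when play begins.
; On BeginPlay it creates a WB_Humans widget, then spawns 100 BP_Human actors at random reachable navigation points around itself, handing each the widget reference.
; It counts the spawns, writes the total to the widget and adds it to the viewport.
; A cast to the BP_GI_Waves game instance is left unconnected.
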(event `self.ReceiveBeginPlay`
  (bind _humanwidgetref (`self.humanwidgetref`))
  (bind _returnvalue (`|CreateWidget` "/Game/Widgets/WB_Humans.WB_Humans_C"))
  (set `self.humanwidgetref` _returnvalue)
  (for _ (range 100)
    (`|SpawnActorFromClass` "/Game/Blueprints/BP_Human.BP_Human_C" (`KismetMathLibrary.MakeTransform` (`NavigationSystemV1.K2_GetRandomReachablePointInRadius` (`self.K2_GetActorLocation`) 7000.0 null null)) "AdjustIfPossibleButAlwaysSpawn" "MultiplyWithRoot" null (`self.humanwidgetref`) null)
    (`/Engine/EditorBlueprintResources/StandardMacros.IncrementInt` (`self.humans`)))
  (set `/Game/Widgets/WB_Humans.humans` (`self.humans`) _humanwidgetref)
  (`UserWidget.AddToViewport` _humanwidgetref 0))

(fn `UserConstructionScript`)