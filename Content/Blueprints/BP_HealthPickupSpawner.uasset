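; Health pickup spawner that periodically places pickups of a configurable class at random points within its SpawnArea bounds.
; BeginPlay starts a randomized-interval timer, re-armed after every TrySpawn attempt, so no Tick is used.
; Each attempt must pass an alive-count cap and a probability roll before spawning.
; AlivePickups increments on each spawn; nothing in this Blueprint decrements it.
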(event `ScheduleNextSpawn`
  (`KismetSystemLibrary.K2_SetTimerDelegate` (`|CreateDelegate` :!event `TrySpawn`) (`KismetMathLibrary.RandomFloatInRange` (`self.IntervalMin`) (`self.IntervalMax`))))

(event `self.ReceiveBeginPlay`
  (`self.ScheduleNextSpawn`))

(event `TrySpawn`
  (bind (_origin _boxextent) (`KismetSystemLibrary.GetComponentBounds` (`self.SpawnArea`)))
  (if (>= (`self.AlivePickups`) (`self.MaxAlivePickups`))
    _
    (elif (not (> (`KismetMathLibrary.RandomFloatInRange` 0.0 1.0) (`self.SpawnChance`)))
      (`|SpawnActorFromClass` (`self.PickupClass`) (`KismetMathLibrary.MakeTransform` (`KismetMathLibrary.RandomPointInBoundingBox` _origin _boxextent)) "Undefined" "MultiplyWithRoot" null null)
      (set `self.AlivePickups` (+ (`self.AlivePickups`) 1))))
  (`self.ScheduleNextSpawn`))

(fn `UserConstructionScript`)