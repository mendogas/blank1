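; BP_LevelTimer is a Blueprint that counts elapsed seconds in a level and puts a WB_Timer widget on screen.
; BeginPlay creates the widget for player 0, starts a looping one-second timer by event and also calls EV_UpdateTimerUI once immediately.
; That event only increments ElapsedTime by one.
; UpdateTimerUI is empty and the text-formatting and start-time nodes are unconnected, so this Blueprint never writes the time to the widget.
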(event `self.ReceiveBeginPlay`
  (bind _returnvalue (`|CreateWidget` "/Game/Widgets/WB_Timer.WB_Timer_C" (`GameplayStatics.GetPlayerController` 0)))
  (set `self.TimerWidget` _returnvalue)
  (`UserWidget.AddToViewport` (`self.TimerWidget`) 0)
  (`KismetSystemLibrary.K2_SetTimerDelegate` (`|CreateDelegate` :!event `EV_UpdateTimerUI`) 1.0 true)
  (`self.EV_UpdateTimerUI`))

(event `EV_UpdateTimerUI`
  (set `self.ElapsedTime` (+ (`self.ElapsedTime`) 1.0)))

(fn `UpdateTimerUI`)

(fn `UserConstructionScript`)